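; RTS player controller that drives the camera pawn, marquee unit selection, building placement and unit orders.
; BeginPlay caches camera, game state and HUD references, then spawns the construction preview, construction master and main HUD.
; Primary action selects units or places affordable, non-overlapping buildings paid in wood and ore; secondary cancels placement or issues AI move and target orders by hit actor class.
; Debug-style keys spawn warriors and harvesters at the cursor.
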(event Custom|UpdateSelection
  ;[1 1 1] Update Selection
  (if (Variables|Boolean|GetisHoldingInput)
    (Variables|Marquee|SetHoldingTime (+ (Variables|Marquee|GetHoldingTime) (Variables|Marquee|GetDelta%20Seconds) 0.0))
    (Class|RTSMarqueeSelectionIF|OnInputHold(Message) (Variables|References|GetMarqueeRef))))

(event Custom|Send%20Occupants
  (params (Building :type RTS%20Building%20Master%20BP%20Object%20Reference) (Target%20Unit :type RTS%20Unit%20Master%20Object%20Reference))
  ;[1 1 1] Send Occuoants
  (Default|GetUnit Building Target%20Unit)
  (if (Utilities|Array|ContainsItem (Variables|UnitControl|GetSelected%20Units) Target%20Unit)
    (Utilities|Array|RemoveItem (Variables|UnitControl|GetSelected%20Units) Target%20Unit)
    (if (>= (Utilities|Array|LastIndex (Variables|UnitControl|GetSelected%20Units)) 0)
      (Variables|Boolean|SetIsUnitSelected true)
      (else
        (Variables|Boolean|SetIsUnitSelected false)))))

(event EventBeginPlay
  ;[1 1 1] BeginPlay
  (Utilities|FlowControl|Sequence
    (:then_0
      (Utilities|ReferenceCast) ; Should be first
    )
    (:then_1
      (bind _returnvalue (Game|SpawnActorfromClass "/Game/RTS_Myself/Blueprints/Buildings/RTS_PreviewBuilding_BP.RTS_PreviewBuilding_BP_C" (Variables|ConstructionVariables|GetEmpty%20Transform) "AlwaysSpawn" 0 self 0))
      (Variables|References|SetConstruction%20Preview%20Ref _returnvalue)
      (bind _returnvalue_2 (Game|SpawnActorfromClass "/Game/RTS_Myself/Blueprints/Buildings/RTS_ConstructionMaster_BP.RTS_ConstructionMaster_BP_C" (Variables|ConstructionVariables|GetEmpty%20Transform) "Undefined" 0 self 0))
      (Variables|References|SetConstructionMasterRef _returnvalue_2))
    (:then_2
      (Utilities|SpawnWidgets)
      (UserInterface|Viewport|AddtoViewport (Variables|References|GetHUD_Main_Ref) 1)
      (HUD|SetHUDVisibility "Visible" "Visible"))
    (:then_3
      (Input|SetInputModeGameandUI self 0 "DoNotLock" false))))

(event EventTick
  (params (DeltaSeconds :type Float%20%28single-precision%29))
  ;[1 1 1] Tick
  (Variables|Marquee|SetDelta%20Seconds DeltaSeconds)
  (if (Variables|Boolean|GetisHoldingInput)
    (CallFunction|UpdateSelection)
    (elif (and (Variables|Boolean|GetisBuildingModeActive) (Utilities|IsValid (Variables|References|GetConstruction%20Preview%20Ref)))
      (Default|GetCursorPosition (Variables|References|GetConstruction%20Preview%20Ref) (CallFunction|SetCursorWorldPosition self 1e+04)))))

(event Input|ActionEvents|InputActionHideBars
  (params (Key :type Key%20Structure))
  ;[1 1 1] Hide Bars
  (:Pressed
    (bind _output_get (Variables|Default|SetShowBars (+ (Variables|Default|GetShowBars) 1)))
    (if (== _output_get 3)
      (Variables|Default|SetShowBars 0))))

(event Input|ActionEvents|InputActionZoomIn
  (params (Key :type Key%20Structure))
  (bind _camerapawnref (Variables|References|GetCameraPawnRef))
  (bind _springarm (Variables|/Game/RTS_Myself/Blueprints/Player/RTS_CameraPawn_BP.RTS_CameraPawn_BP_C|GetSpringArm _camerapawnref))
  ;[1 1 1] Zoom
  ;;[1 1 1] Zoom In
  (:Pressed
    (Variables|/Script/Engine.SpringArmComponent|SetTargetArmLength _springarm (Math|Float|Clamp(Float) (- (Variables|/Script/Engine.SpringArmComponent|GetTargetArmLength _springarm) (Variables|MovementVariables|GetZoomSpeed)) (Variables|MovementVariables|GetMinZoomLimit) (Variables|MovementVariables|GetMaxZoomLimit)))))

(event Input|ActionEvents|InputActionRotatePreviewLeft
  (params (Key :type Key%20Structure))
  (bind _construction_preview_ref (Variables|References|GetConstruction%20Preview%20Ref))
  (bind _returnvalue (Transformation|GetActorRotation _construction_preview_ref))
  ;[1 1 1] Rotate Preview
  ;;[1 1 1] Left
  (:Pressed
    (if (and (Variables|Boolean|GetisBuildingModeActive) (Utilities|IsValid _construction_preview_ref))
      (Transformation|SetActorRotation _construction_preview_ref (Math|Rotator|MakeRotator (.roll _returnvalue) (.pitch _returnvalue) (+ (.yaw _returnvalue) (Variables|ConstructionVariables|GetConstructionRotationRate)))))))

(event Input|ActionEvents|InputActionRotatePreviewRight
  (params (Key :type Key%20Structure))
  (bind _construction_preview_ref (Variables|References|GetConstruction%20Preview%20Ref))
  (bind _returnvalue (Transformation|GetActorRotation _construction_preview_ref))
  ;[1 1 1] Rotate Preview
  ;;[1 1 1] Right
  (:Pressed
    (if (and (Variables|Boolean|GetisBuildingModeActive) (Utilities|IsValid _construction_preview_ref))
      (Transformation|SetActorRotation _construction_preview_ref (Math|Rotator|MakeRotator (.roll _returnvalue) (.pitch _returnvalue) (- (.yaw _returnvalue) (Variables|ConstructionVariables|GetConstructionRotationRate)))))))

(event Input|ActionEvents|InputActionZoomOut
  (params (Key :type Key%20Structure))
  (bind _camerapawnref (Variables|References|GetCameraPawnRef))
  (bind _springarm (Variables|/Game/RTS_Myself/Blueprints/Player/RTS_CameraPawn_BP.RTS_CameraPawn_BP_C|GetSpringArm _camerapawnref))
  ;[1 1 1] Zoom
  ;;[1 1 1] Zoom Out
  (:Pressed
    (Variables|/Script/Engine.SpringArmComponent|SetTargetArmLength _springarm (Math|Float|Clamp(Float) (+ (Variables|MovementVariables|GetZoomSpeed) (Variables|/Script/Engine.SpringArmComponent|GetTargetArmLength _springarm)) (Variables|MovementVariables|GetMinZoomLimit) (Variables|MovementVariables|GetMaxZoomLimit)))))

(event Input|ActionEvents|InputActionPan
  (params (Key :type Key%20Structure))
  (bind _camerapawnref (Variables|References|GetCameraPawnRef))
  (bind _returnvalue (Transformation|GetActorRotation _camerapawnref))
  (bind (_roll _pitch _yaw) (Math|Rotator|BreakRotator _returnvalue))
  ;[1 1 1] Pan
  ;;[1 1 1] Pan Up-Down
  (:Pressed
    (Variables|Default|SetbShowMouseCursor false)
    (Utilities|FlowControl|Gate true) ; enters at Open
  )
  (:Released
    (Variables|Default|SetbShowMouseCursor true)
    (Utilities|FlowControl|Gate true) ; enters at Close
  ))

(event Input|ActionEvents|InputActionPanReset
  (params (Key :type Key%20Structure))
  (bind _camerapawnref (Variables|References|GetCameraPawnRef))
  (bind _returnvalue (Transformation|GetActorRotation _camerapawnref))
  (bind (_roll _pitch _yaw) (Math|Rotator|BreakRotator _returnvalue))
  ;[1 1 1] Pan
  ;;[1 1 1] Reset Pan
  (:Pressed
    (Transformation|SetActorRotation _camerapawnref (Math|Rotator|MakeRotator _roll 0.0 _yaw))))

(event Input|ActionEvents|InputActionPan
  (params (Key :type Key%20Structure))
  (bind _camerapawnref (Variables|References|GetCameraPawnRef))
  (bind _returnvalue (Transformation|GetActorRotation _camerapawnref))
  (bind (_roll _pitch _yaw) (Math|Rotator|BreakRotator _returnvalue))
  ;[1 1 1] Pan
  ;;[1 1 1] Pan Left-Right
  (:Pressed
    (Variables|Default|SetbShowMouseCursor false)
    (Utilities|FlowControl|Gate true) ; enters at Open
  )
  (:Released
    (Variables|Default|SetbShowMouseCursor true)
    (Utilities|FlowControl|Gate true) ; enters at Close
  ))

(event Input|ActionEvents|InputActionMovementSpeedModify
  (params (Key :type Key%20Structure))
  ;[1 1 1] SpeedModifier
  (:Pressed
    (Variables|MovementVariables|SetMovementSpeedModifier 3.0))
  (:Released
    (Variables|MovementVariables|SetMovementSpeedModifier 1.0)))

(event Input|ActionEvents|InputActionSecondaryAction
  (params (Key :type Key%20Structure))
  (bind (_hitresult _returnvalue) (Game|Player|GetHitResultUnderCursorbyChannel "TraceTypeQuery1" false))
  (bind _selectableobjectsenum (Variables|HitResult|GetSelectableObjectsEnum))
  (bind _hitresult_2 (Class|PlayerController|GetHitResultUnderCursorforObjects _selectableobjectsenum true))
  ;[1 1 1] Secondary Action
  (:Pressed
    (if (Variables|Boolean|GetisBuildingModeActive)
      (Default|DestroyPreview (Variables|References|GetConstruction%20Preview%20Ref))
      (elif (Variables|Boolean|GetIsUnitSelected)
        (if _returnvalue
          (Variables|UnitMovement|SetTargetLocation (.location _hitresult))
          (Variables|HitResult|SetHit%20Actor (.hitactor (.HitResult (Class|PlayerController|GetHitResultUnderCursorforObjects (Variables|HitResult|GetSelectableObjectsEnum) true))))
          (Utilities|FlowControl|Sequence
            (:then_0
              (Utilities|UnitMovement))))
        (elif (!= (.hitactor _hitresult_2) 0)
          (Default|CallDisplayHUD (.hitactor _hitresult_2) false)
          (Variables|Default|SetbShowMouseCursor true))))))

(event Input|ActionEvents|InputActionPrimaryAction
  (params (Key :type Key%20Structure))
  ;[1 1 1] Primary Action
  (:Pressed
    (if (Variables|Boolean|GetisBuildingModeActive)
      (if (CallFunction|CheckResources)
        (if (not (Default|CheckOverlap (Variables|References|GetConstruction%20Preview%20Ref)))
          (CallFunction|ReduceResources)
          (bind _construction_struct (Default|SetConstructionStructure (Variables|References|GetConstruction%20Preview%20Ref)))
          (Default|StartConstruction (Variables|References|GetConstructionMasterRef) _construction_struct)
          (Default|DestroyPreview (Variables|References|GetConstruction%20Preview%20Ref)))
        (else
          (Default|TriggerNoFundsText (Variables|References|GetHUD_Main_Ref))))
      (else
        (Class|RTSMarqueeSelectionIF|OnInputStart(Message) (Variables|References|GetMarqueeRef))
        (Variables|Marquee|SetHoldingTime 0.0)
        (Variables|Boolean|SetisHoldingInput true))))
  (:Released
    (if (not (Variables|Boolean|GetisBuildingModeActive))
      (Class|RTSMarqueeSelectionIF|OnInputRelease(Message) (Variables|References|GetMarqueeRef) (Variables|Marquee|GetHoldingTime))
      (Variables|Boolean|SetisHoldingInput false))))

(event Input|ActionEvents|InputActionZoomReset
  (params (Key :type Key%20Structure))
  ;[1 1 1] Zoom
  ;;[1 1 1] Reset Zoom
  (:Pressed
    (Variables|/Script/Engine.SpringArmComponent|SetTargetArmLength (Variables|/Game/RTS_Myself/Blueprints/Player/RTS_CameraPawn_BP.RTS_CameraPawn_BP_C|GetSpringArm (Variables|References|GetCameraPawnRef)) 1.5e+03)))

(event Input|AxisEvents|InputAxisMoveForward
  (params (AxisValue :type Float%20%28single-precision%29))
  (bind _camerapawnref (Variables|References|GetCameraPawnRef))
  (bind _returnvalue (Transformation|GetActorLocation _camerapawnref))
  ;[1 1 1] Camera Keys Movement
  (Transformation|AddActorLocalOffset (Variables|References|GetCameraPawnRef) (Math|Vector|MakeVector (* AxisValue (Variables|MovementVariables|GetDefaultMovementSpeed) (Variables|MovementVariables|GetMovementSpeedModifier)) 0.0 0.0) true false)
  (Transformation|SetActorLocation _camerapawnref (Math|Vector|MakeVector (.x _returnvalue) (.y _returnvalue) 1e+01) true false))

(event Input|AxisEvents|InputAxisMoveRight
  (params (AxisValue :type Float%20%28single-precision%29))
  (bind _camerapawnref (Variables|References|GetCameraPawnRef))
  (bind _returnvalue (Transformation|GetActorLocation _camerapawnref))
  ;[1 1 1] Camera Keys Movement
  (Transformation|AddActorLocalOffset (Variables|References|GetCameraPawnRef) (Math|Vector|MakeVector 0.0 (* AxisValue (Variables|MovementVariables|GetDefaultMovementSpeed) (Variables|MovementVariables|GetMovementSpeedModifier)) 0.0) true false)
  (Transformation|SetActorLocation _camerapawnref (Math|Vector|MakeVector (.x _returnvalue) (.y _returnvalue) 1e+01) true false))

(event Input|MouseEvents|MouseX
  (params (AxisValue :type Float%20%28single-precision%29))
  (bind _camerapawnref (Variables|References|GetCameraPawnRef))
  (bind _returnvalue (Transformation|GetActorRotation _camerapawnref))
  (bind (_roll _pitch _yaw) (Math|Rotator|BreakRotator _returnvalue))
  ;[1 1 1] Pan
  ;;[1 1 1] Pan Left-Right
  (Utilities|FlowControl|Gate true
    (:Exit
      (Transformation|SetActorRotation _camerapawnref (Math|Rotator|MakeRotator 0.0 _pitch (+ _yaw (* AxisValue (Variables|MovementVariables|GetPanSpeed))))))))

(event Input|MouseEvents|MouseY
  (params (AxisValue :type Float%20%28single-precision%29))
  (bind _camerapawnref (Variables|References|GetCameraPawnRef))
  (bind _returnvalue (Transformation|GetActorRotation _camerapawnref))
  (bind (_roll _pitch _yaw) (Math|Rotator|BreakRotator _returnvalue))
  ;[1 1 1] Pan
  ;;[1 1 1] Pan Up-Down
  (Utilities|FlowControl|Gate true
    (:Exit
      (Transformation|SetActorRotation _camerapawnref (Math|Rotator|MakeRotator 0.0 (Math|Float|Clamp(Float) (+ _pitch (* AxisValue (Variables|MovementVariables|GetPanSpeed))) -2e+01 5e+01) _yaw)))))

(event Input|MouseEvents|MouseX
  (params (AxisValue :type Float%20%28single-precision%29))
  (bind _camerapawnref (Variables|References|GetCameraPawnRef))
  (bind _returnvalue (Transformation|GetActorLocation _camerapawnref))
  ;[1 1 1] EdgeScroll
  (if (Variables|Default|GetbShowMouseCursor)
    (bind (_deltaspeedx _deltaspeedy) (Utilities|EdgeScroll))
    (Transformation|AddActorLocalOffset (Variables|References|GetCameraPawnRef) (Math|Vector|MakeVector _deltaspeedx _deltaspeedy 0.0) true false)
    (Transformation|SetActorLocation _camerapawnref (Math|Vector|MakeVector (.x _returnvalue) (.y _returnvalue) 1e+01) true false)))

(event Input|MouseEvents|MouseY
  (params (AxisValue :type Float%20%28single-precision%29))
  (bind _camerapawnref (Variables|References|GetCameraPawnRef))
  (bind _returnvalue (Transformation|GetActorLocation _camerapawnref))
  ;[1 1 1] EdgeScroll
  (if (Variables|Default|GetbShowMouseCursor)
    (Utilities|EdgeScroll) ; enters at Mouse Y
  ))

(event Input|KeyboardEvents|V
  (params (Key :type Key%20Structure))
  (bind _self self)
  (bind _relativecursorlocationingame (CallFunction|SetCursorWorldPosition _self 1e+04))
  ;[1 1 1] Spawn
  ;;[1 1 1] Spawn Warrior
  (:Pressed
    (Game|SpawnActorfromClass "/Game/RTS_Myself/Units/RTS_WarriorUnit.RTS_WarriorUnit_C" (Math|Transform|MakeTransform (Math|Vector|MakeVector (.x _relativecursorlocationingame) (.y _relativecursorlocationingame) 2e+02)) "AdjustIfPossibleButAlwaysSpawn" 0 5e+01 1.0 0)))

(event Input|KeyboardEvents|B
  (params (Key :type Key%20Structure))
  (bind _self self)
  (bind _relativecursorlocationingame (CallFunction|SetCursorWorldPosition _self 1e+04))
  ;[1 1 1] Spawn
  ;;[1 1 1] Spawn Worker
  (:Pressed
    (Game|SpawnActorfromClass "/Game/RTS_Myself/Units/RTS_HarvesterUnit.RTS_HarvesterUnit_C" (Math|Transform|MakeTransform (Math|Vector|MakeVector (.x _relativecursorlocationingame) (.y _relativecursorlocationingame) 2e+02)) "AdjustIfPossibleButAlwaysSpawn" 0 1.0 0)))

(fn ConstructionScript)

(fn SetHUDVisibility
  (params (GameTimeHUD :type ESlateVisibility%20Enum :default "Visible") (ResourcesHUD :type ESlateVisibility%20Enum :default "Visible"))
  (Widget|SetVisibility (Variables|References|GetHUD_Main_Ref) GameTimeHUD))

(fn SetSelectedUnits
  (params (SelectedUnits :type Array%20of%20RTS%20Unit%20Master%20Object%20References) (SelectedVehicles :type Array%20of%20RTS%20Ground%20Vehicle%20Master%20Object%20References))
  (Variables|UnitControl|SetSelected%20Units SelectedUnits)
  (Variables|UnitControl|SetSelected%20Vehicles SelectedVehicles)
  (if (or (>= (Utilities|Array|LastIndex (Variables|UnitControl|GetSelected%20Units)) 0) (>= (Utilities|Array|LastIndex SelectedVehicles) 0))
    (Variables|Boolean|SetIsUnitSelected true)))

(fn SetBuildingModeActive
  (params (is%20Active :type Boolean))
  (Variables|Boolean|SetisBuildingModeActive is%20Active)
  (return))

(fn CheckResources
  (bind _construction_preview_ref (Variables|References|GetConstruction%20Preview%20Ref))
  (return (and (>= (Variables|Resources|GetWoodResource) (Variables|/Game/RTS_Myself/Blueprints/Buildings/RTS_PreviewBuilding_BP.RTS_PreviewBuilding_BP_C|GetWood%20Cost _construction_preview_ref)) (>= (Variables|Resources|GetOreResource) (Variables|/Game/RTS_Myself/Blueprints/Buildings/RTS_PreviewBuilding_BP.RTS_PreviewBuilding_BP_C|GetOre%20Cost _construction_preview_ref)))))

(fn ReduceResources
  (bind _construction_preview_ref (Variables|References|GetConstruction%20Preview%20Ref))
  (Variables|Resources|SetWoodResource (- (Variables|Resources|GetWoodResource) (Variables|/Game/RTS_Myself/Blueprints/Buildings/RTS_PreviewBuilding_BP.RTS_PreviewBuilding_BP_C|GetWood%20Cost _construction_preview_ref)))
  (Variables|Resources|SetOreResource (- (Variables|Resources|GetOreResource) (Variables|/Game/RTS_Myself/Blueprints/Buildings/RTS_PreviewBuilding_BP.RTS_PreviewBuilding_BP_C|GetOre%20Cost _construction_preview_ref)))
  (return))

(fn ReturnResources
  (params (Wood%20Amount :type Float%20%28double-precision%29) (Ore%20Amount :type Float%20%28double-precision%29))
  (Variables|Resources|SetWoodResource (+ (Variables|Resources|GetWoodResource) Wood%20Amount))
  (Variables|Resources|SetOreResource (+ (Variables|Resources|GetOreResource) Ore%20Amount))
  (return))

(fn UpdateBuildingList
  (bind _outactors (Actor|GetAllActorsOfClass "/Game/RTS_Myself/Blueprints/Buildings/RTS_BuildingMaster_BP.RTS_BuildingMaster_BP_C"))
  (for _array_element _outactors
    (if (Variables|/Game/RTS_Myself/Blueprints/Buildings/RTS_BuildingMaster_BP.RTS_BuildingMaster_BP_C|GetisBuilt _array_element)
      (Utilities|Array|AddUnique (Variables|Default|GetListOfConstructedBuildings) _array_element)
      (if (== (Utilities|GetClass _array_element) "/Game/RTS_Myself/Blueprints/Buildings/ResourceManagement/RTS_Silo_BP.RTS_Silo_BP_C")
        (Utilities|Array|AddUnique (Variables|Default|GetSilosList) _array_element))))
  (return))