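; RTS HUD that implements drag-box (marquee) selection of units and ground vehicles.
; Input start clears the previous selection and anchors the rectangle at the cursor, and hold updates its far corner.
; While dragging, DrawHUD draws a green box and uses GetActorsInSelectionRectangle to add or remove units and vehicles live, toggling decals and skipping enemy units.
; Input release passes both selection arrays to the RTS player controller.
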(event Custom|DrawMarquee
  (bind _startlocation (Variables|Default|GetStartLocation))
  (bind _holdinglocation (Variables|Default|GetHoldingLocation))
  (bind _returnvalue (- _holdinglocation _startlocation))
  (bind (_x _y) (Math|Vector2D|BreakVector2D _startlocation))
  (HUD|DrawRect "(R=0.000000,G=1.000000,B=0.000000,A=0.498039)" _x _y (.x _returnvalue) (.y _returnvalue)))

(event EventBeginPlay
  (Variables|References|SetControllerRef (.AsRTS%20Player%20Controller%20BP (Utilities|Casting|CastToRTS_PlayerController_BP (Game|GetPlayerController 0)))))

(event EventOnInputStart
  (bind _controllerref (Variables|References|GetControllerRef))
  (bind (_locationx _locationy) (Game|Player|GetMousePosition _controllerref))
  (if (or (>= (Utilities|Array|LastIndex (Variables|Units|GetSelectedUnits)) 0) (>= (Utilities|Array|LastIndex (Variables|Default|GetSelected%20Ground%20Vehicles)) 0))
    (Utilities|FlowControl|Sequence
      (:then_0
        (for _array_element (Variables|Units|GetSelectedUnits)
          (Default|SetDeselectedDecal _array_element)
          (Variables|/Game/RTS_Myself/Units/RTS_UnitMaster.RTS_UnitMaster_C|SetIs%20Selected _array_element false)
          (Variables|/Game/RTS_Myself/Blueprints/Player/RTS_PlayerController_BP.RTS_PlayerController_BP_C|SetIsUnitSelected (Variables|References|GetControllerRef) false))
        (Utilities|Array|Clear (Variables|Units|GetSelectedUnits)))
      (:then_1
        (for _array_element_2 (Variables|Default|GetSelected%20Ground%20Vehicles)
          (Default|SetDeselectedDecal _array_element_2)
          (Variables|/Game/RTS_Myself/Units/GroundVehicle/RTS_GroundVehicle_Master.RTS_GroundVehicle_Master_C|SetisSelected _array_element_2 false)
          (Variables|/Game/RTS_Myself/Blueprints/Player/RTS_PlayerController_BP.RTS_PlayerController_BP_C|SetIsUnitSelected (Variables|References|GetControllerRef) false))
        (Utilities|Array|Clear (Variables|Default|GetSelected%20Ground%20Vehicles)))
      (:then_2
        (bind _output_get (Variables|Default|SetStartLocation (Math|Vector2D|MakeVector2D _locationx _locationy) :!label _label))
        (Variables|Default|SetHoldingLocation _output_get)
        (Variables|Default|SetIsDrawing true)))
    (else
      (goto _label))))

(event EventOnInputRelease
  (params (HoldTime :type Float%20%28double-precision%29))
  (Variables|Default|SetIsDrawing false)
  (Default|SetSelectedUnits (Variables|References|GetControllerRef) (Variables|Units|GetSelectedUnits) (Variables|Default|GetSelected%20Ground%20Vehicles)))

(event EventDrawHUD
  (params (SizeX :type Integer) (SizeY :type Integer))
  (bind _selectedunits (Variables|Units|GetSelectedUnits))
  (bind _selected_ground_vehicles (Variables|Default|GetSelected%20Ground%20Vehicles))
  (if (Variables|Default|GetIsDrawing)
    (Utilities|FlowControl|Sequence
      (:then_0
        (CallFunction|DrawMarquee))
      (:then_1
        (bind _output_get (Variables|Units|SetUnitsInSelectionArea (Class|HUD|GetActorsinSelectionRectangle "/Game/RTS_Myself/Units/RTS_UnitMaster.RTS_UnitMaster_C" (Variables|Default|GetStartLocation) (Variables|Default|GetHoldingLocation) false false)))
        (for _array_element _output_get
          (if (Utilities|ClassIsChildOf (Utilities|GetClass _array_element) "/Game/RTS_Myself/Units/RTS_UnitMaster.RTS_UnitMaster_C")
            (if (not (Utilities|ClassIsChildOf (Utilities|GetClass _array_element) "/Game/RTS_Myself/Units/Enemy/RTS_Enemy_Master.RTS_Enemy_Master_C"))
              (bind _asrts_unit_master (Utilities|Casting|CastToRTS_UnitMaster _array_element))
              (Utilities|FlowControl|Sequence
                (:then_0
                  (Utilities|Array|AddUnique _selectedunits _asrts_unit_master))
                (:then_1
                  (for _array_element_2 _selectedunits
                    (Default|SetSelectedDecal _array_element_2)
                    (Variables|/Game/RTS_Myself/Units/RTS_UnitMaster.RTS_UnitMaster_C|SetIs%20Selected _array_element_2 true)))))))
        (for _array_element_3 (Variables|Units|GetSelectedUnits)
          (Utilities|IsValid _array_element_3
            (:Is%20Valid
              (bind _asactor (Utilities|Casting|CastToActor _array_element_3))
              (if (not (Utilities|Array|ContainsItem (Variables|Units|GetUnitsInSelectionArea) _asactor))
                (Default|SetDeselectedDecal _array_element_3)
                (Variables|/Game/RTS_Myself/Units/RTS_UnitMaster.RTS_UnitMaster_C|SetIs%20Selected _array_element_3 false)
                (Utilities|Array|RemoveItem (Variables|Units|GetSelectedUnits) _array_element_3))))))
      (:then_2
        (bind _output_get_2 (Variables|Default|SetGround%20Vehicles%20in%20Selection%20Area (Class|HUD|GetActorsinSelectionRectangle "/Game/RTS_Myself/Units/GroundVehicle/RTS_GroundVehicle_Master.RTS_GroundVehicle_Master_C" (Variables|Default|GetStartLocation) (Variables|Default|GetHoldingLocation) false false)))
        (for _array_element_4 _output_get_2
          (if (Utilities|ClassIsChildOf (Utilities|GetClass _array_element_4) "/Game/RTS_Myself/Units/GroundVehicle/RTS_GroundVehicle_Master.RTS_GroundVehicle_Master_C")
            (bind _asrts_ground_vehicle_master (Utilities|Casting|CastToRTS_GroundVehicle_Master _array_element_4))
            (Utilities|FlowControl|Sequence
              (:then_0
                (Utilities|Array|AddUnique _selected_ground_vehicles _asrts_ground_vehicle_master))
              (:then_1
                (for _array_element_5 _selected_ground_vehicles
                  (Default|SetSelectedDecal _array_element_5)
                  (Variables|/Game/RTS_Myself/Units/GroundVehicle/RTS_GroundVehicle_Master.RTS_GroundVehicle_Master_C|SetisSelected _array_element_5 true))))))
        (for _array_element_6 (Variables|Default|GetSelected%20Ground%20Vehicles)
          (bind _asactor_2 (Utilities|Casting|CastToActor _array_element_6))
          (if (not (Utilities|Array|ContainsItem (Variables|Default|GetGround%20Vehicles%20in%20Selection%20Area) _asactor_2))
            (Default|SetDeselectedDecal _array_element_6)
            (Variables|/Game/RTS_Myself/Units/GroundVehicle/RTS_GroundVehicle_Master.RTS_GroundVehicle_Master_C|SetisSelected _array_element_6 false)
            (Utilities|Array|RemoveItem (Variables|Default|GetSelected%20Ground%20Vehicles) _array_element_6)))))))

(event EventOnInputHold
  (bind _controllerref (Variables|References|GetControllerRef))
  (bind (_locationx _locationy) (Game|Player|GetMousePosition _controllerref))
  (Variables|Default|SetHoldingLocation (Math|Vector2D|MakeVector2D _locationx _locationy)))

(fn ConstructionScript)