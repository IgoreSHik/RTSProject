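; Level actor that turns the sun to follow the RTS game clock.
; BeginPlay caches the RTS game state.
; Each tick it reads the game time, yaws the referenced sun 15 degrees per time unit from an offset at a fixed downward pitch, then refreshes the sky sphere's sun direction.
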(event EventBeginPlay
  (Variables|References|SetGameStateRef (.AsRTS%20Game%20State%20BP (Utilities|Casting|CastToRTS_GameState_BP (Game|GetGameState)))))

(event EventTick
  (params (DeltaSeconds :type Float%20%28single-precision%29))
  (bind _gametime (Default|GetGameTime (Variables|References|GetGameStateRef)))
  (Transformation|SetActorRotation (Variables|References|GetSunRef) (Math|Rotator|MakeRotator 0.0 -5e+01 (+ (* _gametime 15.0) 55.0)))
  (Default|UpdateSunDirection (Variables|References|GetSkySphereRef)))

(fn ConstructionScript)