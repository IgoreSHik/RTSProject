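; RTS game state that runs the in-game clock and calendar, seeded from the system date and time on BeginPlay.
; Tick advances time by game speed, updates the HUD and switches the camera pawn's spotlight on outside 8:00–20:00.
; A day rollover advances the calendar and runs a birthday check on every RTS_UnitMaster.
; Speed changes scale the default game speed by a multiplier and pass it to GameSpeedControl.
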(event EventBeginPlay
  (bind _returnvalue (Math|DateTime|Now))
  (bind (_year _month _day _hour _minute _second) (Math|DateTime|BreakDateTime _returnvalue))
  (Utilities|FlowControl|Sequence
    (:then_0
      (Utilities|ReferenceCast))
    (:then_1
      (Variables|Calendar|SetYear _year)
      (Variables|Calendar|SetMonth _month)
      (Variables|Calendar|SetDay _day)
      (Variables|Clock|SetHours _hour)
      (Variables|Clock|SetMinutes _minute)
      (Variables|Clock|SetSeconds _second))
    (:then_2
      (Variables|GameSpeedSettings|SetGameTime (+ (Math|Conversions|ToFloat(Integer) (Variables|Clock|GetHours)) (/ (Math|Conversions|ToFloat(Integer) (Variables|Clock|GetMinutes)) 6e+01) (/ (Math|Conversions|ToFloat(Integer) (Variables|Clock|GetSeconds)) 3.6e+03)))
      (Variables|Calendar|SetGameDate (Utilities|Array|MakeArray (Variables|Calendar|GetDay) (Variables|Calendar|GetMonth) (Variables|Calendar|GetYear))))
    (:then_3
      (Variables|GameSpeedSettings|SetGameSpeed (Variables|GameSpeedSettings|GetDefaultGameSpeed)))))

(event EventTick
  (params (DeltaSeconds :type Float%20%28single-precision%29))
  (Variables|GameSpeedSettings|SetGameTime (.GameTime (CallFunction|SetGameTime DeltaSeconds (Variables|GameSpeedSettings|GetGameSpeed) (Variables|GameSpeedSettings|GetGameTime))))
  (Variables|Calendar|SetDayCounter (.DayCount (CallFunction|SetGameTime DeltaSeconds (Variables|GameSpeedSettings|GetGameSpeed) (Variables|GameSpeedSettings|GetGameTime))))
  (CallFunction|SetClock)
  (CallFunction|SetCalendar)
  (if (== (.DayCount (CallFunction|SetGameTime DeltaSeconds (Variables|GameSpeedSettings|GetGameSpeed) (Variables|GameSpeedSettings|GetGameTime))) 1)
    (bind _unitsout (CallFunction|GetAllUnits))
    (for _array_element _unitsout
      (Default|BirthdayCheck _array_element))))

(event EventFuncUpdateGameSpeed
  (params (SpeedMultiplier :type Float%20%28double-precision%29))
  (bind _output_get (Variables|GameSpeedSettings|SetSpeedMultiplayer SpeedMultiplier))
  (bind _output_get_2 (Variables|GameSpeedSettings|SetGameSpeed (* _output_get (Variables|GameSpeedSettings|GetDefaultGameSpeed))))
  (Default|CallGameSpeedControl _output_get_2))

(fn ConstructionScript)

(fn SetClock
  (bind _gametime (Variables|GameSpeedSettings|GetGameTime))
  (bind _conrollerref (Variables|References|GetConrollerRef))
  (bind _returnvalue (* _gametime 3.6e+03))
  (bind _camerapawnref (Variables|/Game/RTS_Myself/Blueprints/Player/RTS_PlayerController_BP.RTS_PlayerController_BP_C|GetCameraPawnRef _conrollerref))
  (bind (_remainder _returnvalue_2) (Math|Float|Division(WholeandRemainder) _returnvalue 6e+01))
  (bind _spotlight (Variables|/Game/RTS_Myself/Blueprints/Player/RTS_CameraPawn_BP.RTS_CameraPawn_BP_C|GetSpotLight _camerapawnref))
  (bind _returnvalue_3 (Math|Conversions|ToFloat(Integer) _returnvalue_2))
  (bind (_remainder_2 _returnvalue_4) (Math|Float|Division(WholeandRemainder) _returnvalue_3 6e+01))
  (Variables|Clock|SetSeconds (Math|Float|Floor _remainder))
  (Variables|Clock|SetMinutes (Math|Float|Floor _remainder_2))
  (Variables|Clock|SetHours (Math|Float|Floor (.Remainder (Math|Float|Division(WholeandRemainder) (Math|Conversions|ToFloat(Integer) _returnvalue_4) 24.0))))
  (bind _output_get (Variables|Calendar|SetGameDate (Utilities|Array|MakeArray (Variables|Clock|GetSeconds) (Variables|Clock|GetMinutes) (Variables|Clock|GetHours))))
  (Class|RTSGameTimeIF|SetGameClock(Message) (Variables|/Game/RTS_Myself/Blueprints/Player/RTS_PlayerController_BP.RTS_PlayerController_BP_C|GetHUD_Main_Ref (Variables|References|GetConrollerRef)) _output_get)
  (if (Math|Integer|InRange(Integer) (Variables|Clock|GetHours) 8 20 true false)
    (Rendering|SetVisibility _spotlight false false)
    (else
      (Rendering|SetVisibility _spotlight true false))))

(fn SetCalendar
  (bind _output_get (Variables|Calendar|SetDay (+ (Variables|Calendar|GetDay) (Variables|Calendar|GetDayCounter))))
  (if (> _output_get (Class|KismetMathLibrary|DaysinMonth (Variables|Calendar|GetYear) (Variables|Calendar|GetMonth)))
    (Variables|Calendar|SetDay 1)
    (Variables|Calendar|SetMonth (+ (Variables|Calendar|GetMonth) 1)))
  (if (> (Variables|Calendar|GetMonth) 12)
    (Variables|Calendar|SetMonth 1)
    (Variables|Calendar|SetYear (+ (Variables|Calendar|GetYear) 1)))
  (bind _output_get_2 (Variables|Calendar|SetGameDate (Utilities|Array|MakeArray (Variables|Calendar|GetDay) (Variables|Calendar|GetMonth) (Variables|Calendar|GetYear))))
  (Class|RTSGameTimeIF|SetGameCalendar(Message) (Variables|/Game/RTS_Myself/Blueprints/Player/RTS_PlayerController_BP.RTS_PlayerController_BP_C|GetHUD_Main_Ref (Variables|References|GetConrollerRef)) _output_get_2))

(fn GetGameSpeed
  (return (Variables|GameSpeedSettings|GetGameSpeed)))

(fn GetGameTime
  (return (Variables|GameSpeedSettings|GetGameTime)))

(fn GetAllUnits
  (bind _outactors (Actor|GetAllActorsOfClass "/Game/RTS_Myself/Units/RTS_UnitMaster.RTS_UnitMaster_C"))
  (bind _output_get (Variables|Default|SetList%20Of%20All%20Units _outactors))
  (return _output_get))

(fn SetGameCalendar
  (params (GameDate :type Array%20of%20Integers))
  (return false))

(fn SetGameClock
  (params (GameTime :type Array%20of%20Integers))
  (return false))