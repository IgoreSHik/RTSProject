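; RTS military training post building that queues recruitment requests and spawns builder, healer, warrior or harvester units.
; RecruitmentTrigger adds the unit type to a queue and sets a looping timer at the training time.
; SpawnNewUnit spawns the front entry's class, notifies it that training is complete and removes it from the queue.
; CheckTrainingQueue clears the timer on an empty queue, but nothing in this graph calls it.
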(event EventBeginPlay
  (|CallParentFunction)
  (Variables|Default|SetTraining%20Time 2.0))

(event Collision|EventActorBeginOverlap
  (params (OtherActor :type Actor%20Object%20Reference))
  (|CallParentFunction OtherActor) ; This node is disabled and will not be called.\nDrag off pins to build functionality.
)

(event EventTick
  (params (DeltaSeconds :type Float%20%28single-precision%29))
  (|CallParentFunction DeltaSeconds) ; This node is disabled and will not be called.\nDrag off pins to build functionality.
)

(event EventRecruitmentTrigger
  (params (Type :type UnitTypes_Enum%20Enum :default "NewEnumerator4"))
  (Utilities|Array|Add (Variables|Default|GetUnitsToBeSpawnedTypes) Type)
  (bind _returnvalue (Utilities|Time|SetTimerbyFunctionName 0 "SpawnNewUnit" (Variables|Default|GetTraining%20Time) true))
  (Variables|Default|SetSpawnUnitTimerHandle _returnvalue))

(fn ConstructionScript
  (|CallParentFunction))

(fn SpawnNewUnit
  (switch Utilities|FlowControl|Switch|SwitchonUnitTypes_Enum (Utilities|Array|Get(acopy) (Variables|Default|GetUnitsToBeSpawnedTypes))
    (:NewEnumerator0
      (bind _returnvalue (Game|SpawnActorfromClass "/Game/RTS_Myself/Units/RTS_BuilderUnit.RTS_BuilderUnit_C" (Utilities|SpawnTransform) "AdjustIfPossibleButAlwaysSpawn" 0 1.0 0))
      (Default|OnTrainingComplete _returnvalue))
    (:NewEnumerator1
      (bind _returnvalue_2 (Game|SpawnActorfromClass "/Game/RTS_Myself/Units/RTS_HealerUnit.RTS_HealerUnit_C" (Utilities|SpawnTransform) "AdjustIfPossibleButAlwaysSpawn" 0 1.0 0))
      (Default|OnTrainingComplete _returnvalue_2))
    (:NewEnumerator2
      (bind _returnvalue_3 (Game|SpawnActorfromClass "/Game/RTS_Myself/Units/RTS_WarriorUnit.RTS_WarriorUnit_C" (Utilities|SpawnTransform) "AdjustIfPossibleButAlwaysSpawn" 0 5e+01 1.0 0))
      (Default|OnTrainingComplete _returnvalue_3))
    (:NewEnumerator3
      (bind _returnvalue_4 (Game|SpawnActorfromClass "/Game/RTS_Myself/Units/RTS_HarvesterUnit.RTS_HarvesterUnit_C" (Utilities|SpawnTransform) "AdjustIfPossibleButAlwaysSpawn" 0 1.0 0))
      (Default|OnTrainingComplete _returnvalue_4)))
  (Utilities|Array|RemoveIndex (Variables|Default|GetUnitsToBeSpawnedTypes)))

(fn CheckTrainingQueue
  (if (Utilities|Array|IsEmpty (Variables|Default|GetUnitsToBeSpawnedTypes))
    (Utilities|Time|ClearandInvalidateTimerbyHandle (Variables|Default|GetSpawnUnitTimerHandle)))
  (return))