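; Base RTS building that houses units, gets built over game time and shows its own info HUD.
; While units are inside an unfinished building, Tick accumulates work time from game speed and occupant count, then restores materials, releases occupants and updates the controller's building list.
; The construction script applies a preview material until built and sizes the entry box, whose overlap signals arrival to units targeting this building.
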(event OnComponentBeginOverlap(EntryPoint)
  (params (OverlappedComponent :type Primitive%20Component%20Object%20Reference) (OtherActor :type Actor%20Object%20Reference) (OtherComp :type Primitive%20Component%20Object%20Reference) (OtherBodyIndex :type Integer) (bFromSweep :type Boolean) (SweepResult :type Hit%20Result%20Structure%20%28by%20ref%29))
  ;[1 1 1] Common to all buildings
  (bind _asrts_unit_master (Utilities|Casting|CastToRTS_UnitMaster OtherActor))
  (bind _output_get (Variables|Default|SetOverlaping%20Unit _asrts_unit_master))
  (if (== (Variables|/Game/RTS_Myself/Units/RTS_UnitMaster.RTS_UnitMaster_C|GetTarget%20Building _output_get) self)
    (Default|ArriveatBuilding (Variables|Default|GetOverlaping%20Unit))))

(event Custom|OnSpawn
  ;[1 1 1] Common to all buildings
  (Variables|Bool|SetisUnderConstruction true))

(event Custom|Recruitment%20Trigger
  (params (Type :type UnitTypes_Enum%20Enum :default "NewEnumerator4")))

(event Custom|Get%20Game%20Speed
  (params (GameTime :type Float%20%28double-precision%29))
  ;[1 1 1] Common to all buildings
  (Variables|Construction|SetGame%20Speed GameTime))

(event Custom|Display%20Building%20HUD
  (params (Actor :type Actor%20Object%20Reference) (Bypass :type Boolean))
  (bind _playercontrollerref (Variables|References|GetPlayerControllerRef))
  ;[1 1 1] Common to all buildings
  (if (== Actor self)
    (UserInterface|Viewport|AddtoViewport (Variables|References|GetBuilding%20HUD) 1)
    (Input|SetInputModeUIOnly _playercontrollerref 0 "DoNotLock" false)
    (Widget|SetIsEnabled (Variables|/Game/RTS_Myself/Blueprints/Player/RTS_PlayerController_BP.RTS_PlayerController_BP_C|GetHUD_Main_Ref _playercontrollerref) true)))

(event EventBeginPlay
  ;[1 1 1] Common to all buildings
  (Utilities|FlowControl|Sequence
    (:then_0
      (Utilities|ReferenceCasts))
    (:then_1
      (EventDispatchers|BindEventtoGameSpeedControl (Variables|References|GetGameStateRef) (delegate Custom|Get%20Game%20Speed))
      (bind _gamespeed (Default|GetGameSpeed (Variables|References|GetGameStateRef)))
      (Variables|Construction|SetGame%20Speed _gamespeed))
    (:then_2
      (EventDispatchers|BindEventtoDisplayHUD (Variables|References|GetPlayerControllerRef) (EventDispatchers|CreateEvent :!event Custom|Display%20Building%20HUD)))))

(event Collision|EventActorBeginOverlap
  (params (OtherActor :type Actor%20Object%20Reference)))

(event EventTick
  (params (DeltaSeconds :type Float%20%28single-precision%29))
  ;[1 1 1] Common to all buildings
  (Variables|Construction|SetDeltaTime DeltaSeconds)
  (if (Math|Boolean|ANDBoolean (Variables|Bool|GetisUnderConstruction) (not (Variables|Bool|GetisBuilt)) (Utilities|Array|IsNotEmpty (Variables|Default|GetUnitsInBuilding)))
    (CallFunction|СonstructBuilding)
    (if (>= (Variables|Construction|GetWorkedTime) (Variables|Construction|GetConstructionTime))
      (Variables|Bool|SetisBuilt true)
      (Variables|Bool|SetisUnderConstruction false)
      (Utilities|ResetMaterials)
      (CallFunction|ReleaseEveryone)
      (Default|UpdateBuildingList (Variables|References|GetPlayerControllerRef)))))

(fn ConstructionScript
  (Components|StaticMesh|SetStaticMesh (Variables|Default|GetBuildingMesh) (Variables|Default|GetDisplayMesh))
  (Variables|Components|SetStandartMaterials (Rendering|Material|GetMaterials (Variables|Default|GetBuildingMesh)))
  (Components|Box|SetBoxExtent (Variables|Default|GetEntryPoint) (.Max (Components|StaticMesh|GetLocalBounds (Variables|Default|GetBuildingMesh))) true)
  (if (Variables|Bool|GetisBuilt)
    (Utilities|ResetMaterials)
    (else
      (for (_ _array_index) (Rendering|Material|GetMaterials (Variables|Default|GetBuildingMesh))
        (Rendering|Material|SetMaterial (Variables|Default|GetBuildingMesh) _array_index "/Game/RTS_Myself/Materials/Construction/Preview_M.Preview_M")))))

(fn GetUnit
  (params (TargetUnit :type RTS%20Unit%20Master%20Object%20Reference))
  (Utilities|Array|AddUnique (Variables|Default|GetUnitsInBuilding) TargetUnit)
  (CallFunction|UpdateUnitsList)
  (return))

(fn ReleaseEveryone
  (bind _unitsinbuilding (Variables|Default|GetUnitsInBuilding))
  (while (Utilities|Array|IsNotEmpty _unitsinbuilding)
    (CallFunction|ReleaseSingle (Utilities|Array|Get(acopy) _unitsinbuilding))))

(fn ReleaseSingle
  (params (Unit :type RTS%20Unit%20Master%20Object%20Reference))
  (Default|LeaveBuilding Unit)
  (Utilities|Array|RemoveItem (Variables|Default|GetUnitsInBuilding) Unit)
  (CallFunction|UpdateUnitsList)
  (return))

(fn UpdateUnitsList
  (Class|RTSOccupantInfoIF|SetOccupantNames(Message) (Variables|References|GetBuilding%20HUD) (Variables|Default|GetUnitsInBuilding))
  (Default|UpdateOccupantList (Variables|References|GetBuilding%20HUD)))

(fn СonstructBuilding
  (bind _output_get (Variables|Construction|SetGame%20Time (+ (.GameTime (CallFunction|SetGameTime (Variables|Construction|GetDeltaTime) (/ (Variables|Construction|GetGame%20Speed) (Utilities|Array|Length (Variables|Default|GetUnitsInBuilding))) (Variables|Construction|GetGame%20Time))) (* (.DayCount (CallFunction|SetGameTime (Variables|Construction|GetDeltaTime) (/ (Variables|Construction|GetGame%20Speed) (Utilities|Array|Length (Variables|Default|GetUnitsInBuilding))) (Variables|Construction|GetGame%20Time))) 24))))
  (Variables|Construction|SetWorkedTime (* _output_get (Variables|Construction|GetConstruction%20Modifier)))
  (return))

(fn SetOccupantNames
  (params (Units :type Array%20of%20RTS%20Unit%20Master%20Object%20References))
  (return false))