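; RTS building placement preview actor that shows a ghost mesh of the selected building and toggles building mode on the player controller.
; ConstructBuilding briefly spawns the building class to read its mesh, name, time and costs, then destroys it.
; While previewing, a gated Tick snaps the ghost to a grid at the cursor position and swaps good/bad materials on actor overlap.
; It also packs the placement into a construction struct, and cancelling parks it below the world.
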(event Custom|DestroyPreview
  (CallFunction|CloseGate)
  (Variables|Default|SetBuilding%20Class 0)
  (Variables|Default|SetDisplay%20Mesh 0)
  (bind _output_get (Variables|Default|SetisPreviewing false))
  (Default|SetBuildingModeActive (Variables|References|GetPlayerControllerRef) _output_get)
  (Transformation|SetActorLocation "0, 0,-1000.000000" false false))

(event Custom|Spawn%20Preview
  (params (BuildingClass :type RTS%20Building%20Master%20BP%20Class%20Reference) (DisplayMesh :type Static%20Mesh%20Object%20Reference) (ConstuctionTime :type Float%20%28double-precision%29) (BuildingName :type BuildingNamesEnum%20Enum :default "NewEnumerator0") (WoodCost :type Float%20%28double-precision%29) (OreCost :type Float%20%28double-precision%29))
  (if (Variables|Default|GetisPreviewing)
    (CallFunction|DestroyPreview))
  (CallFunction|SetBuildingDetails BuildingClass DisplayMesh ConstuctionTime BuildingName WoodCost OreCost)
  (bind _output_get (Variables|Default|SetisPreviewing true))
  (Default|SetBuildingModeActive (Variables|References|GetPlayerControllerRef) _output_get)
  (Components|StaticMesh|SetStaticMesh (Variables|Default|GetPreviewBuildingMesh) (Variables|Default|GetDisplay%20Mesh))
  (CallFunction|OpenGate))

(event Custom|OpenGate
  (bind _previewbuildingmesh (Variables|Default|GetPreviewBuildingMesh))
  (bind _returnvalue (Rendering|Material|GetMaterials _previewbuildingmesh))
  (Utilities|FlowControl|Gate true) ; enters at Open
)

(event Custom|CloseGate
  (bind _previewbuildingmesh (Variables|Default|GetPreviewBuildingMesh))
  (bind _returnvalue (Rendering|Material|GetMaterials _previewbuildingmesh))
  (Utilities|FlowControl|Gate true) ; enters at Close
)

(event EventConstructBuilding
  (params (BuildingMasterClass :type RTS%20Building%20Master%20BP%20Class%20Reference))
  (bind _returnvalue (Game|SpawnActorfromClass BuildingMasterClass (Variables|Default|GetEmpty%20Transform) "AlwaysSpawn" (Variables|References|GetPlayerControllerRef) 0 false "NewEnumerator0" 0))
  (Utilities|FlowControl|Sequence
    (:then_0
      (bind _asrts_building_master_bp (Utilities|Casting|CastToRTS_BuildingMaster_BPClass BuildingMasterClass))
      (CallFunction|DestroyPreview)
      (CallFunction|SpawnPreview _asrts_building_master_bp (Variables|/Game/RTS_Myself/Blueprints/Buildings/RTS_BuildingMaster_BP.RTS_BuildingMaster_BP_C|GetDisplayMesh _returnvalue) (Variables|/Game/RTS_Myself/Blueprints/Buildings/RTS_BuildingMaster_BP.RTS_BuildingMaster_BP_C|GetConstructionTime _returnvalue) (Variables|/Game/RTS_Myself/Blueprints/Buildings/RTS_BuildingMaster_BP.RTS_BuildingMaster_BP_C|GetBuldingName _returnvalue) (Variables|/Game/RTS_Myself/Blueprints/Buildings/RTS_BuildingMaster_BP.RTS_BuildingMaster_BP_C|GetWoodCost _returnvalue) (Variables|/Game/RTS_Myself/Blueprints/Buildings/RTS_BuildingMaster_BP.RTS_BuildingMaster_BP_C|GetOreCost _returnvalue)))
    (:then_1
      (Actor|DestroyActor _returnvalue))))

(event EventTick
  (params (DeltaSeconds :type Float%20%28single-precision%29))
  (bind _previewbuildingmesh (Variables|Default|GetPreviewBuildingMesh))
  (bind _returnvalue (Rendering|Material|GetMaterials _previewbuildingmesh))
  (Utilities|FlowControl|Gate true
    (:Exit
      (Transformation|SetActorLocation self (CallFunction|GridSnap) false false)
      (if (CallFunction|CheckOverlap)
        (for (_ _array_index) _returnvalue
          (Rendering|Material|SetMaterial _previewbuildingmesh _array_index "/Game/RTS_Myself/Materials/Construction/PreviewBad_M_Inst.PreviewBad_M_Inst"))
        (else
          (for (_ _array_index_2) _returnvalue
            (Rendering|Material|SetMaterial _previewbuildingmesh _array_index_2 "/Game/RTS_Myself/Materials/Construction/PreviewGod_M_Inst.PreviewGod_M_Inst")))))))

(fn ConstructionScript)

(fn GetCursorPosition
  (params (CursorPositionIn :type Vector))
  (Variables|Default|SetCursorWorldPosition CursorPositionIn)
  (return))

(fn GridSnap
  (bind _cursorworldposition (Variables|Default|GetCursorWorldPosition))
  (bind _snapvalue (Variables|Default|GetSnapValue))
  (bind _snapvalue_2 (Variables|Default|GetSnapValue))
  (return (Math|Vector|MakeVector (* (Math|Float|Round (/ (.x _cursorworldposition) _snapvalue_2)) _snapvalue_2) (* (Math|Float|Round (/ (.y _cursorworldposition) _snapvalue)) _snapvalue) (.z _cursorworldposition))))

(fn CheckOverlap
  (return (>= (Utilities|Array|LastIndex (Collision|GetOverlappingActors 0 :!class /Script/Engine.Actor)) 0)))

(fn SetConstructionStructure
  (bind _output_get (Variables|Default|SetConstructionStruct (Utilities|Struct|MakeRTS_Construction_Struct false (Variables|Default|GetBuilding%20Class) (Math|Transform|MakeTransform (Transformation|GetActorLocation) (Transformation|GetActorRotation)) (Variables|Default|GetDisplay%20Mesh) (Variables|Default|GetConstruction%20Time) (Variables|Default|GetBuilding%20Name))))
  (return _output_get))

(fn SetBuildingDetails
  (params (Building%20Class :type RTS%20Building%20Master%20BP%20Class%20Reference) (Display%20Mesh :type Static%20Mesh%20Object%20Reference) (Construction%20Time :type Float%20%28double-precision%29) (Building%20Name :type BuildingNamesEnum%20Enum :default "NewEnumerator0") (Wood%20Cost :type Float%20%28double-precision%29) (Ore%20Cost :type Float%20%28double-precision%29))
  (Variables|Default|SetBuilding%20Class Building%20Class)
  (Variables|Default|SetDisplay%20Mesh Display%20Mesh)
  (Variables|Default|SetConstruction%20Time Construction%20Time)
  (Variables|Default|SetBuilding%20Name Building%20Name)
  (Variables|Default|SetWood%20Cost Wood%20Cost)
  (Variables|Default|SetOre%20Cost Ore%20Cost))