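; Spawn volume that places resource actors at random points within its bounds in an RTS, on begin play and/or on a repeating timer.
; SpawnResource box-traces each random point and spawns only when the hit actor is Landscape.
; Tick derives the interval from TimeSetting and GameState game speed, restarting the timer on change.
; Timed spawns skip while the HUD is paused; MaxResourcesSpawned is checked only at begin play.
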(event Custom|SpawnResourcesOnTimer
  (if (not (Variables|/Game/RTS_Myself/Blueprints/Widgets/MainPlayer_HUD.MainPlayer_HUD_C|GetIsPaused (Variables|/Game/RTS_Myself/Blueprints/Player/RTS_PlayerController_BP.RTS_PlayerController_BP_C|GetHUD_Main_Ref (Variables|References|GetPlayerControllerRef))))
    (if (Variables|Default|GetIsSpawnedOnTimer)
      (CallFunction|SpawnResource (Variables|References|GetResourceRef) (Variables|Resources|GetNumberOfResourcesSpawned))
      (Variables|Resources|SetTotalNumberSpawned (+ (Variables|Resources|GetNumberOfResourcesSpawned) (Variables|Resources|GetTotalNumberSpawned))))))

(event Custom|GetGameSpeed
  (params (GameSpeed :type Float%20%28double-precision%29))
  (Variables|Resources|SetGame%20Speed GameSpeed))

(event EventBeginPlay
  (Utilities|FlowControl|Sequence
    (:then_0
      (Utilities|RefCastMacro))
    (:then_1
      (EventDispatchers|BindEventtoGameSpeedControl (Variables|References|GetGameStateRef) (EventDispatchers|CreateEvent :!event Custom|GetGameSpeed))
      (bind _gamespeed (Default|GetGameSpeed (Variables|References|GetGameStateRef)))
      (Variables|Resources|SetGame%20Speed _gamespeed)
      (CallFunction|SetRespawnTimer))
    (:then_2
      (if (Variables|Default|GetIsSpawnedOnBeginPlay)
        (CallFunction|SpawnResource (Variables|References|GetResourceRef) (Variables|Resources|GetNumberOfResourcesSpawned))
        (Variables|Resources|SetTotalNumberSpawned (+ (Variables|Resources|GetNumberOfResourcesSpawned) (Variables|Resources|GetTotalNumberSpawned)))
        (if (and (Variables|Default|GetIsSpawnedOnTimer) (< (Variables|Resources|GetTotalNumberSpawned) (Variables|Resources|GetMaxResourcesSpawned)))
          (Utilities|Time|SetTimerbyEvent (EventDispatchers|CreateEvent :!event Custom|SpawnResourcesOnTimer) (Variables|Resources|GetRespawnTime) true))))))

(event Collision|EventActorBeginOverlap
  (params (OtherActor :type Actor%20Object%20Reference)))

(event EventTick
  (params (DeltaSeconds :type Float%20%28single-precision%29))
  (CallFunction|SetRespawnTimer)
  (if (not (== (Variables|Resources|GetRespawnTime) (Variables|Resources|GetRespawnTimer)))
    (Variables|Resources|SetRespawnTimer (Variables|Resources|GetRespawnTime))
    (Utilities|Time|SetTimerbyEvent (EventDispatchers|CreateEvent :!event Custom|SpawnResourcesOnTimer) (Variables|Resources|GetRespawnTime) true)))

(fn ConstructionScript)

(fn SpawnResource
  (params (Resource :type RTS%20Resource%20Master%20BP%20Class%20Reference) (SpawnAmount :type Integer))
  (bind (_origin _boxextent) (Collision|GetActorBounds false false))
  (bind _z (Math|Vector|BreakVector _origin))
  (bind _returnvalue (* (.y _boxextent) 2.0))
  (bind _returnvalue_2 (* (.x _boxextent) 2.0))
  (bind _returnvalue_3 (- (.x _boxextent) _returnvalue_2))
  (bind _returnvalue_4 (- (.y _boxextent) _returnvalue))
  (bind _returnvalue_5 (Math|Random|RandomFloatinRange _returnvalue_3 (.x _boxextent)))
  (bind _returnvalue_6 (Math|Random|RandomFloatinRange _returnvalue_4 (.y _boxextent)))
  (bind _returnvalue_7 (Math|Vector|MakeVector _returnvalue_5 _returnvalue_6 _z))
  (bind _returnvalue_8 (+ _origin _returnvalue_7))
  (bind _returnvalue_9 (Math|Vector|MakeVector (.x _returnvalue_8) (.y _returnvalue_8) 1e+02))
  (LocalVariables|SetResourceRefLocal Resource)
  (bind _output_get (LocalVariables|SetSpawnAmountLocal SpawnAmount))
  (for _index (range 1 _output_get)
    (bind _outhit (Collision|BoxTraceByChannel _returnvalue_9 "0, 0, 0" _returnvalue_9 "0, 0, 0" "TraceTypeQuery1" false 0 "None"))
    (if (== (Utilities|GetClass (.HitActor (Collision|BreakHitResult _outhit))) "/Script/Landscape.Landscape")
      (Game|SpawnActorfromClass (LocalVariables|GetResourceRefLocal) (Math|Conversions|ToTransform(Vector) (.Location (Collision|BreakHitResult _outhit))) "Undefined" 0 false false true 0.5 1.1 0))))

(fn SetRespawnTimer
  (switch Utilities|FlowControl|Switch|SwitchonRespawnTimer_Enum (Variables|References|GetTimeSetting)
    (:NewEnumerator1
      (Variables|Resources|SetRespawnTime 0.0))
    (:NewEnumerator2
      (Variables|Resources|SetRespawnTime (Variables|Resources|GetGame%20Speed)))
    (:NewEnumerator3
      (Variables|Resources|SetRespawnTime (Variables|Resources|GetUserRespawnTimer)))
    (:NewEnumerator4
      (Variables|Resources|SetRespawnTime (* (Variables|Resources|GetUserRespawnTimer) (Variables|Resources|GetGame%20Speed)))))
  (return (Variables|Resources|GetRespawnTime)))