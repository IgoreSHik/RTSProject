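; RTS wood resource Blueprint, placed in the world as a harvestable tree node.
; Its construction script runs the parent construction, sets the resource mesh to a random pick from four generic tree meshes, then calls AfterConstruction.
; The event graph holds only disabled default events, so any other behavior comes from the parent class.
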(event EventBeginPlay
  (|CallParentFunction) ; This node is disabled and will not be called.\nDrag off pins to build functionality.
)

(event Collision|EventActorBeginOverlap
  (params (OtherActor :type Actor%20Object%20Reference))
  (|CallParentFunction OtherActor) ; This node is disabled and will not be called.\nDrag off pins to build functionality.
)

(event EventTick
  (params (DeltaSeconds :type Float%20%28single-precision%29))
  (|CallParentFunction DeltaSeconds) ; This node is disabled and will not be called.\nDrag off pins to build functionality.
)

(fn ConstructionScript
  (|CallParentFunction)
  (Components|StaticMesh|SetStaticMesh (Variables|Default|GetResourceMesh) (.OutItem (Utilities|Array|Random (Utilities|Array|MakeArray "/Game/PolygonTown/Meshes/Generic/SM_Generic_Tree_01.SM_Generic_Tree_01" "/Game/PolygonTown/Meshes/Generic/SM_Generic_Tree_02.SM_Generic_Tree_02" "/Game/PolygonTown/Meshes/Generic/SM_Generic_Tree_03.SM_Generic_Tree_03" "/Game/PolygonTown/Meshes/Generic/SM_Generic_Tree_04.SM_Generic_Tree_04"))))
  (CallFunction|AfterConstruction))