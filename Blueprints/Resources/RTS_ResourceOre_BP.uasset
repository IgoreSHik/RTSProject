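; RTS_ResourceOre_BP is an ore resource actor for an RTS, extending a parent resource Blueprint.
; Its construction script calls the parent's, sets ResourceMesh to a randomly picked small stone mesh, then calls AfterConstruction.
; The event graph holds only disabled default events, so this asset adds no runtime logic of its own.
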(event EventBeginPlay
  (|CallParentFunction) ; This node is disabled and will not be called.\nDrag off pins to build functionality.
)

(event Collision|EventActorBeginOverlap
  (params (OtherActor :type Actor%20Object%20Reference))
  (|CallParentFunction OtherActor) ; This node is disabled and will not be called.\nDrag off pins to build functionality.
)

(event EventTick
  (params (DeltaSeconds :type Float%20%28single-precision%29))
  (|CallParentFunction DeltaSeconds) ; This node is disabled and will not be called.\nDrag off pins to build functionality.
)

(fn ConstructionScript
  (|CallParentFunction)
  (Components|StaticMesh|SetStaticMesh (Variables|Default|GetResourceMesh) (.OutItem (Utilities|Array|Random (Utilities|Array|MakeArray "/Game/DreamscapeSeries/DreamscapeMeadows/Meshes/Rocks/SM_Stone_Small_03.SM_Stone_Small_03" "/Game/DreamscapeSeries/DreamscapeMeadows/Meshes/Rocks/SM_Stone_Small_04.SM_Stone_Small_04" "/Game/DreamscapeSeries/DreamscapeMeadows/Meshes/Rocks/SM_Stone_Small_05.SM_Stone_Small_05" "/Game/DreamscapeSeries/DreamscapeMeadows/Meshes/Rocks/SM_Stone_Small_06.SM_Stone_Small_06"))))
  (CallFunction|AfterConstruction))