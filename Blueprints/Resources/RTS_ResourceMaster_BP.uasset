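; Master Blueprint for RTS resource nodes that harvester units gather from and deplete.
; Construction sets resource amount from level (optionally random) and random size, with optional mesh scaling and yaw, saving original amount and scale only when random rotation is on.
; Harvester overlap on ResourceEntry calls HarvestTrigger and marks the node busy until Tick times out.
; ChangeSize shrinks the mesh with remaining resources, destroying the actor when empty.
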(event OnComponentBeginOverlap(ResourceEntry)
  (params (OverlappedComponent :type Primitive%20Component%20Object%20Reference) (OtherActor :type Actor%20Object%20Reference) (OtherComp :type Primitive%20Component%20Object%20Reference) (OtherBodyIndex :type Integer) (bFromSweep :type Boolean) (SweepResult :type Hit%20Result%20Structure%20%28by%20ref%29))
  (bind _asrts_harvester_unit (Utilities|Casting|CastToRTS_HarvesterUnit OtherActor))
  (Default|HarvestTrigger _asrts_harvester_unit)
  (Variables|Default|SetNot%20Harvested%20Time 0.0)
  (Variables|Default|SetIs%20Free false))

(event EventBeginPlay)

(event Collision|EventActorBeginOverlap
  (params (OtherActor :type Actor%20Object%20Reference)))

(event EventTick
  (params (DeltaSeconds :type Float%20%28single-precision%29))
  (bind _output_get (Variables|Default|SetNot%20Harvested%20Time (+ (Variables|Default|GetNot%20Harvested%20Time) (Utilities|Time|GetWorldDeltaSeconds))))
  (if (>= _output_get 1e+01)
    (Variables|Default|SetIs%20Free true)))

(fn ConstructionScript
  (if (Variables|Bool|GetIsRandomLevel)
    (bind _output_get (Variables|References|SetResourceLevelEnumRef (Utilities|Enum|ByteToEnumResourceLevel_Enum (Math|Conversions|ToByte(Integer) (Math|Random|RandomIntegerinRange 1 5))))))
  (switch Utilities|FlowControl|Switch|SwitchonResourceLevel_Enum _output_get
    (:NewEnumerator1
      (Variables|ResourceValue|SetResourceModifier 1.0))
    (:NewEnumerator2
      (Variables|ResourceValue|SetResourceModifier 1.2))
    (:NewEnumerator3
      (Variables|ResourceValue|SetResourceModifier 1.4))
    (:NewEnumerator4
      (Variables|ResourceValue|SetResourceModifier 1.6))
    (:NewEnumerator5
      (Variables|ResourceValue|SetResourceModifier 1.8))
    (:NewEnumerator6
      (Variables|ResourceValue|SetResourceModifier 2.0)))
  (bind _output_get_2 (Variables|Default|SetSize (Math|Random|RandomFloatinRange (Variables|SpawnSize|GetMinMeshSize) (Variables|SpawnSize|GetMaxMeshSize))))
  (Variables|ResourceValue|SetCurrentResources (* (Variables|ResourceValue|GetBaseResourceAmount) (Variables|ResourceValue|GetResourceModifier) _output_get_2))
  (if (Variables|Bool|GetIsRandomSize)
    (Transformation|SetWorldScale3D (Variables|Default|GetResourceMesh) (Math|Vector|MakeVector (Variables|Default|GetSize) (Variables|Default|GetSize) (Variables|Default|GetSize))))
  (if (Variables|Bool|GetIsRandomRotated)
    (Transformation|SetWorldRotation (Variables|Default|GetResourceMesh) (Math|Rotator|MakeRotator 0.0 0.0 (Math|Random|RandomFloatinRange 0.0 3.6e+02)) false false)
    (Variables|Default|SetOriginalResources (Variables|ResourceValue|GetCurrentResources))
    (Variables|Default|SetOriginalScale (Transformation|GetWorldScale (Variables|Default|GetResourceMesh)))))

(fn AfterConstruction
  (Components|Box|SetBoxExtent (Variables|Default|GetResourceEntry) (* (.Max (Components|StaticMesh|GetLocalBounds (Variables|Default|GetResourceMesh))) (Variables|Default|GetSize)) true))

(fn ChangeSize
  (Transformation|SetWorldScale3D (Variables|Default|GetResourceMesh) (* (+ (* (/ (Variables|ResourceValue|GetCurrentResources) (Variables|Default|GetOriginalResources)) 0.9) 0.1) (Variables|Default|GetOriginalScale)))
  (if (<= (Variables|ResourceValue|GetCurrentResources) 0.0)
    (Actor|DestroyActor)))